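; Lever-and-door puzzle test Blueprint where interacting while the screen shows the winning color opens the door.
; A timeline, rate-scaled by the display time, loops the screen through an array of materials.
; A correct interaction stops the cycle, rotates the door and shows the win material.
; A wrong one pauses the cycle and shows the lose material until a second timeline finishes, then resumes.
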(event `self.ReceiveBeginPlay`
  (`TimelineComponent.SetPlayRate` (`self.Timeline`) (/ 1.0 (`self.ScreenTimeDisplay`)))
  (`PrimitiveComponent.SetMaterial` (`self.screen`) 0 (`|GetArrayItem` (`self.MScreenArray`)))
  (`TimelineComponent.SetPlayRate` (`self.TimelineLose`) (/ 1.0 (`self.ScreenTimeDisplayError`)))
  (`self.ChangeColor`))

(event `PlayColor`
  (`Timeline|Timeline` :!label _label
    (:`Finished`
      (if (== (`self.IndexM`) (- (`KismetArrayLibrary.Array_Length` (`self.MScreenArray`)) 1))
        (set `self.IndexM` 0)
        (`PrimitiveComponent.SetMaterial` (`self.screen`) 0 (`|GetArrayItem` (`self.MScreenArray`) (`self.IndexM`)))
        (else
          (set `self.IndexM` (+ (`self.IndexM`) 1))
          (`PrimitiveComponent.SetMaterial` (`self.screen`) 0 (`|GetArrayItem` (`self.MScreenArray`) (`self.IndexM`)))))
      (`self.ChangeColor`))))

(event `ChangeColor`
  (goto _label :!via `PlayFromStart`))

(event `PauseColor`
  (goto _label :!via `Stop`))

(event `/Game/04_Blueprint/IInteractObjects.Interact`
  (params (NewParam :type "Pawn Object Reference"))
  (if (== (`self.IndexWin`) (`self.IndexM`))
    (`SceneComponent.K2_AddWorldRotation` (`self.door`) (`KismetMathLibrary.Quat_Rotator` (`KismetMathLibrary.Quat_MakeFromEuler` (+ (`KismetMathLibrary.Vector_Zero`) (`KismetMathLibrary.MakeVector` 0.0 0.0 (`self.rotationDoorOpen`))))) false false)
    (`self.PauseColor`)
    (`PrimitiveComponent.SetMaterial` (`self.screen`) 0 (`self.MWin`))
    (else
      (`self.PauseColor`)
      (`PrimitiveComponent.SetMaterial` (`self.screen`) 0 (`self.MLose`))
      (`Timeline|TimelineLose`
        (:`Finished`
          (`PrimitiveComponent.SetMaterial` (`self.screen`) 0 (`|GetArrayItem` (`self.MScreenArray`) (`self.IndexM`)))
          (`self.PlayColor`))))))

(fn `UserConstructionScript`)