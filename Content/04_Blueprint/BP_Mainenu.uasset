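; Main menu controller Blueprint that shows and switches between the main and options menu screens in English or French.
; On BeginPlay it reads language and volume from GI_Maps, spawns the matching widget and enables game-and-UI input with a cursor.
; Widgets receive a reference to it; its events swap screens, toggle the language by replacing the options widget, and apply master volume through a sound mix, saving it to the GameInstance.
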(event `self.ReceiveBeginPlay`
  (bind _returnvalue (`GameplayStatics.GetPlayerController` 0))
  (bind _asgi_maps (cast `/Game/04_Blueprint/GI_Maps` (`GameplayStatics.GetGameInstance`)))
  (bind _output_get (set `self.GIRef` _asgi_maps))
  (set `self.soundVolume` (`/Game/04_Blueprint/GI_Maps.volume` _output_get))
  (if (`/Game/04_Blueprint/GI_Maps.IsFrench` (`self.GIRef`))
    (bind _returnvalue_2 (`|CreateWidget` "/Game/04_Blueprint/WidgetMain/WBP_MenuPauseFRMain.WBP_MenuPauseFRMain_C" _returnvalue))
    (bind _output_get_2 (set `self.PauseMenuWidgetFR` _returnvalue_2))
    (`/Game/04_Blueprint/WidgetMain/WBP_MenuPauseFRMain.SetRef` _output_get_2 self)
    (`UserWidget.AddToViewport` _output_get_2 0)
    (`WidgetBlueprintLibrary.SetInputMode_GameAndUIEx` null _returnvalue_2)
    (set `PlayerController.bShowMouseCursor` true _returnvalue)
    (else
      (bind _returnvalue_3 (`|CreateWidget` "/Game/04_Blueprint/WidgetMain/WBP_MenuPauseENMain.WBP_MenuPauseENMain_C" _returnvalue))
      (bind _output_get_3 (set `self.PauseMenuWidget` _returnvalue_3))
      (`/Game/04_Blueprint/WidgetMain/WBP_MenuPauseENMain.SetRef` _output_get_3 self)
      (`UserWidget.AddToViewport` _output_get_3 0)
      (`WidgetBlueprintLibrary.SetInputMode_GameAndUIEx` null _returnvalue_3)
      (set `PlayerController.bShowMouseCursor` true _returnvalue))))

(event `PassFrench`
  (bind _returnvalue (`GameplayStatics.GetPlayerController` 0))
  (if (`/Game/04_Blueprint/GI_Maps.IsFrench` (`self.GIRef`))
    (set `/Game/04_Blueprint/GI_Maps.IsFrench` false (`self.GIRef`))
    (bind _returnvalue_2 (`|CreateWidget` "/Game/04_Blueprint/WidgetMain/WBP_MenuOptionENMain.WBP_MenuOptionENMain_C" _returnvalue))
    (bind _output_get (set `self.OptionMenuWidgetEN` _returnvalue_2))
    (`/Game/04_Blueprint/WidgetMain/WBP_MenuOptionENMain.SetRef` _output_get self)
    (`UserWidget.AddToViewport` _returnvalue_2 0)
    (`Widget.RemoveFromParent` (`self.OptionMenuWidgetFR`))
    (else
      (set `/Game/04_Blueprint/GI_Maps.IsFrench` true (`self.GIRef`))
      (bind _returnvalue_3 (`|CreateWidget` "/Game/04_Blueprint/WidgetMain/WBP_MenuOptionFRMain.WBP_MenuOptionFRMain_C" _returnvalue))
      (bind _output_get_2 (set `self.OptionMenuWidgetFR` _returnvalue_3))
      (`/Game/04_Blueprint/WidgetMain/WBP_MenuOptionFRMain.SetRef` _output_get_2 self)
      (`UserWidget.AddToViewport` _returnvalue_3 0)
      (`Widget.RemoveFromParent` (`self.OptionMenuWidgetEN`)))))

(event `VolumeChange`
  (params (NewVolume :type "Float (double-precision)"))
  (`GameplayStatics.SetSoundMixClassOverride` "/Game/04_Blueprint/WidgetPause/MasterSoundMix.MasterSoundMix" "/Engine/EngineSounds/Master.Master" NewVolume 1.0 0.0)
  (`GameplayStatics.PushSoundMixModifier` "/Game/04_Blueprint/WidgetPause/MasterSoundMix.MasterSoundMix")
  (bind _output_get (set `self.soundVolume` NewVolume))
  (set `/Game/04_Blueprint/GI_Maps.volume` _output_get (`self.GIRef`)))

(event `Back`
  (bind _returnvalue (`GameplayStatics.GetPlayerController` 0))
  (set `self.isOption` false)
  (if (`/Game/04_Blueprint/GI_Maps.IsFrench` (`self.GIRef`))
    (bind _returnvalue_2 (`|CreateWidget` "/Game/04_Blueprint/WidgetMain/WBP_MenuPauseFRMain.WBP_MenuPauseFRMain_C" _returnvalue))
    (bind _output_get (set `self.PauseMenuWidgetFR` _returnvalue_2))
    (`/Game/04_Blueprint/WidgetMain/WBP_MenuPauseFRMain.SetRef` _output_get self)
    (`UserWidget.AddToViewport` _output_get 0)
    (`Widget.RemoveFromParent` (`self.OptionMenuWidgetFR`))
    (else
      (bind _returnvalue_3 (`|CreateWidget` "/Game/04_Blueprint/WidgetMain/WBP_MenuPauseENMain.WBP_MenuPauseENMain_C" _returnvalue))
      (bind _output_get_2 (set `self.PauseMenuWidget` _returnvalue_3))
      (`/Game/04_Blueprint/WidgetMain/WBP_MenuPauseENMain.SetRef` _output_get_2 self)
      (`UserWidget.AddToViewport` _output_get_2 0)
      (`Widget.RemoveFromParent` (`self.OptionMenuWidgetEN`)))))

(event `Option`
  (bind _returnvalue (`GameplayStatics.GetPlayerController` 0))
  (set `self.isOption` true)
  (if (`/Game/04_Blueprint/GI_Maps.IsFrench` (`self.GIRef`))
    (bind _returnvalue_2 (`|CreateWidget` "/Game/04_Blueprint/WidgetMain/WBP_MenuOptionFRMain.WBP_MenuOptionFRMain_C" _returnvalue))
    (bind _output_get (set `self.OptionMenuWidgetFR` _returnvalue_2))
    (`/Game/04_Blueprint/WidgetMain/WBP_MenuOptionFRMain.SetRef` _output_get self)
    (`Widget.RemoveFromParent` (`self.PauseMenuWidgetFR`))
    (`UserWidget.AddToViewport` _returnvalue_2 0)
    (else
      (bind _returnvalue_3 (`|CreateWidget` "/Game/04_Blueprint/WidgetMain/WBP_MenuOptionENMain.WBP_MenuOptionENMain_C" _returnvalue))
      (bind _output_get_2 (set `self.OptionMenuWidgetEN` _returnvalue_3))
      (`/Game/04_Blueprint/WidgetMain/WBP_MenuOptionENMain.SetRef` _output_get_2 self)
      (`Widget.RemoveFromParent` (`self.PauseMenuWidget`))
      (`UserWidget.AddToViewport` _returnvalue_3 0))))

(fn `UserConstructionScript`)