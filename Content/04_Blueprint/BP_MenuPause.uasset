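; Manages the in-game pause menu and its options screen, with separate English and French widgets chosen by the game instance's IsFrench flag.
; The Pause input or PauseGame event toggles game pause, input mode and cursor while showing or removing the current menu.
; Widgets receive a reference to this actor, whose events switch screens, swap language live and apply master volume through a sound mix.
; Language and volume persist in GI_Maps.
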(event `self.ReceiveBeginPlay`
  (bind _asgi_maps (cast `/Game/04_Blueprint/GI_Maps` (`GameplayStatics.GetGameInstance`)))
  (bind _output_get (set `self.GIRef` _asgi_maps))
  (set `self.soundVolume` (`/Game/04_Blueprint/GI_Maps.volume` _output_get)))

(event `InputAction|Pause` :paused true
  (params (Key :type "Key Structure"))
  (bind _returnvalue (`GameplayStatics.GetPlayerController` 0))
  (bind _returnvalue_2 (`GameplayStatics.GetPlayerController` 0))
  (bind _returnvalue_3 (`GameplayStatics.GetPlayerController` 0))
  (bind _returnvalue_4 (`GameplayStatics.GetPlayerController` 0))
  (bind _returnvalue_5 (`GameplayStatics.GetPlayerController` 0))
  (:`Pressed`
    (if (`self.paused`) :!label _label
      (set `self.paused` false)
      (if (`self.isOption`)
        (set `self.isOption` false)
        (`GameplayStatics.SetGamePaused` false)
        (if (`/Game/04_Blueprint/GI_Maps.IsFrench` (`self.GIRef`))
          (`Widget.RemoveFromParent` (`self.OptionMenuWidgetFR`))
          (`WidgetBlueprintLibrary.SetInputMode_GameOnly` _returnvalue_2)
          (set `PlayerController.bShowMouseCursor` false _returnvalue_2)
          (else
            (`Widget.RemoveFromParent` (`self.OptionMenuWidgetEN`))
            (`WidgetBlueprintLibrary.SetInputMode_GameOnly` _returnvalue)
            (set `PlayerController.bShowMouseCursor` false _returnvalue)))
        (else
          (`GameplayStatics.SetGamePaused` false)
          (if (`/Game/04_Blueprint/GI_Maps.IsFrench` (`self.GIRef`))
            (`Widget.RemoveFromParent` (`self.PauseMenuWidgetFR`))
            (`WidgetBlueprintLibrary.SetInputMode_GameOnly` _returnvalue_5)
            (set `PlayerController.bShowMouseCursor` false _returnvalue_5)
            (else
              (`Widget.RemoveFromParent` (`self.PauseMenuWidget`))
              (`WidgetBlueprintLibrary.SetInputMode_GameOnly` _returnvalue_4)
              (set `PlayerController.bShowMouseCursor` false _returnvalue_4)))))
      (else
        (set `self.paused` true)
        (`GameplayStatics.SetGamePaused` true)
        (if (`/Game/04_Blueprint/GI_Maps.IsFrench` (`self.GIRef`))
          (bind _returnvalue_6 (`|CreateWidget` "/Game/04_Blueprint/WidgetPause/WBP_MenuPauseFR.WBP_MenuPauseFR_C" _returnvalue_3))
          (bind _output_get (set `self.PauseMenuWidgetFR` _returnvalue_6))
          (`/Game/04_Blueprint/WidgetPause/WBP_MenuPauseFR.SetRef` _output_get self)
          (`UserWidget.AddToViewport` _output_get 0)
          (`WidgetBlueprintLibrary.SetInputMode_GameAndUIEx` _returnvalue_3 _returnvalue_6)
          (set `PlayerController.bShowMouseCursor` true _returnvalue_3)
          (else
            (bind _returnvalue_7 (`|CreateWidget` "/Game/04_Blueprint/WidgetPause/WBP_MenuPauseEN.WBP_MenuPauseEN_C"))
            (bind _output_get_2 (set `self.PauseMenuWidget` _returnvalue_7))
            (`/Game/04_Blueprint/WidgetPause/WBP_MenuPauseEN.SetRef` _output_get_2 self)
            (`UserWidget.AddToViewport` _output_get_2 0)
            (`WidgetBlueprintLibrary.SetInputMode_GameAndUIEx` _returnvalue_3 _returnvalue_7)
            (set `PlayerController.bShowMouseCursor` true _returnvalue_3)))))))

(event `PauseGame`
  (goto _label))

(event `PassFrench`
  (bind _returnvalue (`GameplayStatics.GetPlayerController` 0))
  (if (`/Game/04_Blueprint/GI_Maps.IsFrench` (`self.GIRef`))
    (set `/Game/04_Blueprint/GI_Maps.IsFrench` false (`self.GIRef`))
    (bind _returnvalue_2 (`|CreateWidget` "/Game/04_Blueprint/WidgetPause/WBP_MenuOptionEN.WBP_MenuOptionEN_C" _returnvalue))
    (bind _output_get (set `self.OptionMenuWidgetEN` _returnvalue_2))
    (`/Game/04_Blueprint/WidgetPause/WBP_MenuOptionEN.SetRef` _output_get self)
    (`UserWidget.AddToViewport` _returnvalue_2 0)
    (`Widget.RemoveFromParent` (`self.OptionMenuWidgetFR`))
    (else
      (set `/Game/04_Blueprint/GI_Maps.IsFrench` true (`self.GIRef`))
      (bind _returnvalue_3 (`|CreateWidget` "/Game/04_Blueprint/WidgetPause/WBP_MenuOptionFR.WBP_MenuOptionFR_C" _returnvalue))
      (bind _output_get_2 (set `self.OptionMenuWidgetFR` _returnvalue_3))
      (`/Game/04_Blueprint/WidgetPause/WBP_MenuOptionFR.SetRef` _output_get_2 self)
      (`UserWidget.AddToViewport` _returnvalue_3 0)
      (`Widget.RemoveFromParent` (`self.OptionMenuWidgetEN`)))))

(event `VolumeChange`
  (params (NewVolume :type "Float (double-precision)"))
  (`GameplayStatics.SetSoundMixClassOverride` "/Game/04_Blueprint/WidgetPause/MasterSoundMix.MasterSoundMix" "/Engine/EngineSounds/Master.Master" NewVolume 1.0 0.0)
  (`GameplayStatics.PushSoundMixModifier` "/Game/04_Blueprint/WidgetPause/MasterSoundMix.MasterSoundMix")
  (bind _output_get (set `self.soundVolume` NewVolume))
  (set `/Game/04_Blueprint/GI_Maps.volume` _output_get (`self.GIRef`)))

(event `Back`
  (bind _returnvalue (`GameplayStatics.GetPlayerController` 0))
  (set `self.isOption` false)
  (if (`/Game/04_Blueprint/GI_Maps.IsFrench` (`self.GIRef`))
    (bind _returnvalue_2 (`|CreateWidget` "/Game/04_Blueprint/WidgetPause/WBP_MenuPauseFR.WBP_MenuPauseFR_C" _returnvalue))
    (bind _output_get (set `self.PauseMenuWidgetFR` _returnvalue_2))
    (`/Game/04_Blueprint/WidgetPause/WBP_MenuPauseFR.SetRef` _output_get self)
    (`UserWidget.AddToViewport` _output_get 0)
    (`Widget.RemoveFromParent` (`self.OptionMenuWidgetFR`))
    (else
      (bind _returnvalue_3 (`|CreateWidget` "/Game/04_Blueprint/WidgetPause/WBP_MenuPauseEN.WBP_MenuPauseEN_C" _returnvalue))
      (bind _output_get_2 (set `self.PauseMenuWidget` _returnvalue_3))
      (`/Game/04_Blueprint/WidgetPause/WBP_MenuPauseEN.SetRef` _output_get_2 self)
      (`UserWidget.AddToViewport` _output_get_2 0)
      (`Widget.RemoveFromParent` (`self.OptionMenuWidgetEN`)))))

(event `Option`
  (bind _returnvalue (`GameplayStatics.GetPlayerController` 0))
  (set `self.isOption` true)
  (if (`/Game/04_Blueprint/GI_Maps.IsFrench` (`self.GIRef`))
    (bind _returnvalue_2 (`|CreateWidget` "/Game/04_Blueprint/WidgetPause/WBP_MenuOptionFR.WBP_MenuOptionFR_C" _returnvalue))
    (bind _output_get (set `self.OptionMenuWidgetFR` _returnvalue_2))
    (`/Game/04_Blueprint/WidgetPause/WBP_MenuOptionFR.SetRef` _output_get self)
    (`Widget.RemoveFromParent` (`self.PauseMenuWidgetFR`))
    (`UserWidget.AddToViewport` _returnvalue_2 0)
    (else
      (bind _returnvalue_3 (`|CreateWidget` "/Game/04_Blueprint/WidgetPause/WBP_MenuOptionEN.WBP_MenuOptionEN_C" _returnvalue))
      (bind _output_get_2 (set `self.OptionMenuWidgetEN` _returnvalue_3))
      (`/Game/04_Blueprint/WidgetPause/WBP_MenuOptionEN.SetRef` _output_get_2 self)
      (`Widget.RemoveFromParent` (`self.PauseMenuWidget`))
      (`UserWidget.AddToViewport` _returnvalue_3 0))))

(fn `UserConstructionScript`)